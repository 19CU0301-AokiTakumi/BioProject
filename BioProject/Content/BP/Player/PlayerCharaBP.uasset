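; PlayerCharaBP is the player character Blueprint, handling per-frame socket tracking, shot camera shake and a zero-health physics change.
; Each Tick it stores the world location of a right middle-finger socket on the mesh in MSocketLocation.
; While the animation status is Shot, it plays PlayerShootShake on the first player controller.
; Within that same branch, depleted HP turns off body physics simulation and sets mesh collision to physics-only.
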(event `self.ReceiveTick`
  (params (DeltaSeconds :type "Float (single-precision)"))
  (bind _mesh (`self.Mesh`))
  (set `self.m_SocketLocation` (`SceneComponent.GetSocketLocation` (`self.Mesh`) "R_Middle1ソケット"))
  (if (`|EnumEquality` (`self.GetAnimStatus`) "Shot")
    (`PlayerController.ClientStartCameraShake` :`self` (`GameplayStatics.GetPlayerController` 0) :`Shake` "/Game/BP/Player/PlayerShootShake.PlayerShootShake_C")
    (if (<= (`.hp` (break `PlayerStatus` (`self.GetPlayerStatus`))) 0)
      (`SkeletalMeshComponent.SetAllBodiesSimulatePhysics` _mesh false)
      (`PrimitiveComponent.SetCollisionEnabled` _mesh "PhysicsOnly"))))

(fn `UserConstructionScript`)