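; Enemy character Blueprint that drops the library room key when it is shot.
; An overlap with an actor tagged Bullet stops its movement and, only once, creates a dynamic body material and spawns LibraryRoomKeyBP at the enemy's transform.
; A timeline then drives the mesh's opacity parameter as a fade, and the actor is destroyed when it finishes.
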(event `self.ReceiveActorBeginOverlap`
  (params (OtherActor :type "Actor Object Reference"))
  (if (`self.ActorHasTag` OtherActor "Bullet")
    (`MovementComponent.StopMovementImmediately` (`self.CharacterMovement`))
    (`/Engine/EditorBlueprintResources/StandardMacros.DoOnce` false
      (:`Completed`
        (`PrimitiveComponent.CreateDynamicMaterialInstance` (`self.Mesh`) 0 "/Game/NewMap/Body.Body" "None")
        (`/Engine/EditorBlueprintResources/StandardMacros.DoOnce` false
          (:`Completed`
            (`|SpawnActorFromClass` "/Game/BP/LibraryRoomKeyBP.LibraryRoomKeyBP_C" (`self.GetTransform`) "Undefined" "OverrideRootScale" null null)
            (bind (_direction _fadetime) (`Timeline|タイムライン_0`)
              (:`Update`
                (`MeshComponent.SetScalarParameterValueOnMaterials` (`self.Mesh`) "opacity" _fadetime))
              (:`Finished`
                (`self.K2_DestroyActor`)))))))))

(event `self.ReceiveTick`
  (params (DeltaSeconds :type "Float (single-precision)")))

(fn `UserConstructionScript`)