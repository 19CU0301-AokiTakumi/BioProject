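; Enemy Blueprint that reacts to headshots, runs physical animation and fades out on death.
; BeginPlay simulates physics on bones below a set bone, driven by PhysicalAnimation.
; Bullet-tagged overlaps on Head set a down flag; Tick caches the Body position and, in Down or Death state, halts movement and consumes the flag via DownPoint.
; Within those states, zero HP triggers a one-time material opacity timeline, then destroys the actor.
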(event `self.Head.OnComponentBeginOverlap`
  (params (OverlappedComponent :type "PrimitiveComponent Object Reference") (OtherActor :type "Actor Object Reference") (OtherComp :type "PrimitiveComponent Object Reference") (OtherBodyIndex :type Integer) (bFromSweep :type Boolean) (SweepResult :type "HitResult Structure (by ref)"))
  (if (`self.ActorHasTag` OtherActor "Bullet")
    (set `self.m_IsDown` true)))

(event `self.ReceiveTick`
  (params (DeltaSeconds :type "Float (single-precision)"))
  (set `self.m_BodyCollisionPos` (`SceneComponent.K2_GetComponentLocation` (`self.Body`)))
  (if (or (`|EnumEquality` (`self.GetEnemyState`) "Death") (`|EnumEquality` (`self.GetEnemyState`) "Down"))
    (`MovementComponent.StopMovementImmediately` (`self.CharacterMovement`))
    (if (`self.m_IsDown`)
      (`self.DownPoint`)
      (set `self.m_IsDown` false)
      (`KismetSystemLibrary.PrintString` "Hello"))
    (if (<= (`.hp` (break `EnemyStatus` (`self.GetEnemyStatus`))) 0)
      (`/Engine/EditorBlueprintResources/StandardMacros.DoOnce` false
        (:`Completed`
          (`PrimitiveComponent.CreateDynamicMaterialInstance` (`self.Mesh`) 0 "/Game/NewMap/Body.Body" "None")
          (bind (_direction _fadetime) (`Timeline|徐々にOpacityを下げる`)
            (:`Update`
              (`MeshComponent.SetScalarParameterValueOnMaterials` (`self.Mesh`) "opacity" _fadetime))
            (:`Finished`
              (`self.K2_DestroyActor`))))))))

(event `self.ReceiveBeginPlay`
  (bind _bonename (`self.BoneName`))
  (bind _physicalanimation (`self.PhysicalAnimation`))
  (`PhysicalAnimationComponent.SetSkeletalMeshComponent` _physicalanimation (`self.Mesh`))
  (`PhysicalAnimationComponent.ApplyPhysicalAnimationSettingsBelow` _physicalanimation _bonename (make `PhysicalAnimationData` false 600.0 500.0 600.0 500.0) false)
  (`SkeletalMeshComponent.SetAllBodiesBelowSimulatePhysics` (`self.Mesh`) _bonename true false))

(fn `UserConstructionScript`)